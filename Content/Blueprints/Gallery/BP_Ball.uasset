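; BP_Ball is a gallery ball that launches itself on spawn and explodes on hit.
; BeginPlay applies a randomized horizontal, fixed upward velocity-change impulse to its sphere.
; Any hit destroys the ball and spawns an explosion effect at the hit location; destroying the other actor is left unconnected.
; On destruction, it increments BallsDestroyed on the player's BP_FirstPersonCharacter.
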(event EventBeginPlay
  ;[1 1 1] Spawner
  (CallFunction|AddImpulse))

(event EventDestroyed
  (CallFunction|CountBallsDestroyed))

(event Collision|EventHit
  (params (MyComp :type Primitive%20Component%20Object%20Reference) (Other :type Actor%20Object%20Reference) (OtherComp :type Primitive%20Component%20Object%20Reference) (bSelfMoved :type Boolean) (HitLocation :type Vector :default "0, 0, 0") (HitNormal :type Vector :default "0, 0, 0") (NormalImpulse :type Vector :default "0, 0, 0") (Hit :type Hit%20Result%20Structure%20%28by%20ref%29))
  ;[1 1 1] Destroy Ball & Projectile
  (CallFunction|SpawnExplosion Other HitLocation))

(fn ConstructionScript)

(fn AddImpulse
  (bind _output_get (Variables|Default|SetImpulse (Math|Vector|MakeVector (Math|Random|RandomFloatinRange (Variables|Default|GetMinXRandomImpulse) (Variables|Default|GetMaxXRandomImpulse)) (Math|Random|RandomFloatinRange (Variables|Default|GetMinYRandomImpulse) (Variables|Default|GetMaxYRandomImpulse)) (Variables|Default|GetUpwardImpulse))))
  (Physics|AddImpulse (Variables|Default|GetSphere) _output_get "None" true))

(fn CountBallsDestroyed
  (bind _asbp_first_person_character (Utilities|Casting|CastToBP_FirstPersonCharacter (Game|GetPlayerCharacter 0)))
  (Variables|/Game/FirstPerson/Blueprints/BP_FirstPersonCharacter.BP_FirstPersonCharacter_C|SetBallsDestroyed _asbp_first_person_character (+ (Variables|/Game/FirstPerson/Blueprints/BP_FirstPersonCharacter.BP_FirstPersonCharacter_C|GetBallsDestroyed _asbp_first_person_character) 1)))

(fn SpawnExplosion
  (params (OtherActor :type Actor%20Object%20Reference) (HitLocation :type Vector))
  (Actor|DestroyActor)
  (Game|SpawnActorfromClass "/Game/StarterContent/Blueprints/Blueprint_Effect_Explosion.Blueprint_Effect_Explosion_C" (Math|Conversions|ToTransform(Vector) HitLocation) "Undefined" 0 0))