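; BP_BouncingBall_ShootDown is a ball target for the ShootDown mode that scores points for the player when destroyed.
; On BeginPlay it launches its sphere with a random velocity-change impulse along negative Y and upward.
; Any Hit event, without checking what was struck, spawns an explosion at the impact, adds the character's BouncingBallDestroy value to TotalPoints, then destroys the ball.
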(event Collision|EventHit
  (params (MyComp :type Primitive%20Component%20Object%20Reference) (Other :type Actor%20Object%20Reference) (OtherComp :type Primitive%20Component%20Object%20Reference) (bSelfMoved :type Boolean) (HitLocation :type Vector :default "0, 0, 0") (HitNormal :type Vector :default "0, 0, 0") (NormalImpulse :type Vector :default "0, 0, 0") (Hit :type Hit%20Result%20Structure%20%28by%20ref%29))
  (CallFunction|DestroyBall (Math|Conversions|ToTransform(Vector) HitLocation)))

(event EventBeginPlay
  (CallFunction|AddImpulseonStart))

(fn ConstructionScript)

(fn DestroyBall
  (params (Transform :type Transform))
  (Game|SpawnActorfromClass "/Game/StarterContent/Blueprints/Blueprint_Effect_Explosion.Blueprint_Effect_Explosion_C" Transform "Undefined" 0 0)
  (bind _asbp_first_person_character (Utilities|Casting|CastToBP_FirstPersonCharacter (Game|GetPlayerCharacter 0)))
  (Variables|/Game/FirstPerson/Blueprints/BP_FirstPersonCharacter.BP_FirstPersonCharacter_C|SetTotalPoints _asbp_first_person_character (+ (Variables|/Game/FirstPerson/Blueprints/BP_FirstPersonCharacter.BP_FirstPersonCharacter_C|GetTotalPoints _asbp_first_person_character) (Variables|/Game/FirstPerson/Blueprints/BP_FirstPersonCharacter.BP_FirstPersonCharacter_C|GetBouncingBallDestroy _asbp_first_person_character)))
  (Actor|DestroyActor))

(fn AddImpulseonStart
  (bind _output_get (Variables|Default|SetImpulse (Math|Vector|MakeVector 0.0 (Math|Random|RandomFloatinRange -1e+03 -2.5e+03) (Math|Random|RandomFloatinRange 3e+02 1.1e+03))))
  (Physics|AddImpulse (Variables|Default|GetSphere) _output_get "None" true))