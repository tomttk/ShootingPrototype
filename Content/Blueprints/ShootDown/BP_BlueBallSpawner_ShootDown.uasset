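; Spawner actor for the ShootDown game that keeps spawning BP_BouncingBall_ShootDown balls at random intervals.
; Tick feeds a Delay randomized between SpawnTimeMin and SpawnTimeMax, which acts as a repeating timer because it ignores re-triggers while pending.
; Each completion calls SpawnBlueBall, which spawns a ball at SpawnPoint0's relative location converted to world space, regardless of collisions.
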(event EventTick
  (params (DeltaSeconds :type Float%20%28single-precision%29))
  (Utilities|FlowControl|Delay (Math|Random|RandomFloatinRange (Variables|Default|GetSpawnTimeMin) (Variables|Default|GetSpawnTimeMax)))
  (CallFunction|SpawnBlueBall))

(fn ConstructionScript)

(fn SpawnBlueBall
  (Game|SpawnActorfromClass "/Game/Blueprints/ShootDown/BP_BouncingBall_ShootDown.BP_BouncingBall_ShootDown_C" (Math|Conversions|ToTransform(Vector) (Math|Transform|TransformLocation (Transformation|GetActorTransform) (Variables|/Script/Engine.SceneComponent|GetRelativeLocation (Variables|Default|GetSpawnPoint0)))) "AlwaysSpawn" 0 0))