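; BP_Ball_ShootDown is a destructible ball target that awards points to the player when shot down.
; Its Hit event decrements health, spawns an explosion at the hit location, and destroys the ball once health drops below zero.
; Hit and destruction points are read from and added to BP_FirstPersonCharacter's TotalPoints.
; The Destroyed event spawns further explosions at the Sphere's relative location transformed by the actor's transform.
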(event EventBeginPlay)

(event Collision|EventActorBeginOverlap
  (params (OtherActor :type Actor%20Object%20Reference)))

(event EventTick
  (params (DeltaSeconds :type Float%20%28single-precision%29)))

(event Collision|EventHit
  (params (MyComp :type Primitive%20Component%20Object%20Reference) (Other :type Actor%20Object%20Reference) (OtherComp :type Primitive%20Component%20Object%20Reference) (bSelfMoved :type Boolean) (HitLocation :type Vector :default "0, 0, 0") (HitNormal :type Vector :default "0, 0, 0") (NormalImpulse :type Vector :default "0, 0, 0") (Hit :type Hit%20Result%20Structure%20%28by%20ref%29))
  (CallFunction|BallHit (Math|Conversions|ToTransform(Vector) HitLocation)))

(event EventDestroyed
  (CallFunction|SpawnExplosionsonDestroyed))

(fn ConstructionScript)

(fn BallHit
  (params (Transform :type Transform))
  (Variables|Default|SetBallHealth (- (Variables|Default|GetBallHealth) 1))
  (bind _output_get (Variables|Default|SetBall%20Transform Transform))
  (Game|SpawnActorfromClass "/Game/StarterContent/Blueprints/Blueprint_Effect_Explosion.Blueprint_Effect_Explosion_C" _output_get "Undefined" 0 0)
  (CallFunction|AddtoPointsBallHit)
  (Math|Integer|CompareInt (Variables|Default|GetBallHealth)
    (:<
      (Actor|DestroyActor)
      (CallFunction|AddtoPointsBallDestroyed))))

(fn AddtoPointsBallHit
  (bind _asbp_first_person_character (Utilities|Casting|CastToBP_FirstPersonCharacter (Game|GetPlayerCharacter 0)))
  (Variables|/Game/FirstPerson/Blueprints/BP_FirstPersonCharacter.BP_FirstPersonCharacter_C|SetTotalPoints _asbp_first_person_character (+ (Variables|/Game/FirstPerson/Blueprints/BP_FirstPersonCharacter.BP_FirstPersonCharacter_C|GetTotalPoints _asbp_first_person_character) (Variables|/Game/FirstPerson/Blueprints/BP_FirstPersonCharacter.BP_FirstPersonCharacter_C|GetBallPointsHit _asbp_first_person_character))))

(fn AddtoPointsBallDestroyed
  (bind _asbp_first_person_character (Utilities|Casting|CastToBP_FirstPersonCharacter (Game|GetPlayerCharacter 0)))
  (Variables|/Game/FirstPerson/Blueprints/BP_FirstPersonCharacter.BP_FirstPersonCharacter_C|SetTotalPoints _asbp_first_person_character (+ (Variables|/Game/FirstPerson/Blueprints/BP_FirstPersonCharacter.BP_FirstPersonCharacter_C|GetTotalPoints _asbp_first_person_character) (Variables|/Game/FirstPerson/Blueprints/BP_FirstPersonCharacter.BP_FirstPersonCharacter_C|GetBallPointsDestroyed _asbp_first_person_character))))

(fn SpawnExplosionsonDestroyed
  (for _index (range 0 1)
    (Game|SpawnActorfromClass "/Game/StarterContent/Blueprints/Blueprint_Effect_Explosion.Blueprint_Effect_Explosion_C" (Math|Conversions|ToTransform(Vector) (Math|Transform|TransformLocation (Transformation|GetActorTransform) (Variables|/Script/Engine.SceneComponent|GetRelativeLocation (Variables|Default|GetSphere)))) "Undefined" 0 0)))